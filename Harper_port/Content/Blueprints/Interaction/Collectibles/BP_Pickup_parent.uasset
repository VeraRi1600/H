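; BP_Pickup_parent is the base Blueprint for collectible item pickups.
; On overlap it prints a debug string, then checks that the other actor implements an interface and is not itself a pickup.
; It sends that actor a PickupItemMessage with its item class, icon and stack size, then destroys itself.
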(event Collision|EventActorBeginOverlap
  (params (OtherActor :type Actor%20Object%20Reference))
  ;[1 1 1] Is overlaping with PC?
  (Development|PrintString "Hello")
  (if (Utilities|DoesObjectImplementInterface OtherActor 0)
    (if (not (Utilities|ClassIsChildOf (Utilities|GetClass OtherActor) "BP_Pickup_parent_C"))
      (Class|PickupItemInterface|PickupItem(Message) OtherActor (Variables|Default|GetItemClass) (Variables|Default|GetItemIcon) (Variables|Default|GetStackSize))
      (Actor|DestroyActor))))

(fn ConstructionScript)